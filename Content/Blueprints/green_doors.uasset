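; Greenhouse door actor that the first-person character swings open by pressing E.
; Actor overlaps toggle player input on the actor, while a Box overlap with BP_FirstPersonCharacter sets the flag that gates the key.
; A Timeline yaws the door mesh and a SceneCaptureComponent2D up to a scaled angle in opposite directions.
; The creepy opening sound plays only once, and no closing logic exists.
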(event `self.ReceiveBeginPlay`
  (set `self.opened` false)
  (set `self.colliding` false))

(event `self.ReceiveActorBeginOverlap`
  (params (OtherActor :type "Actor Object Reference"))
  (`self.EnableInput` (`GameplayStatics.GetPlayerController` 0)))

(event `self.ReceiveActorEndOverlap`
  (params (OtherActor :type "Actor Object Reference"))
  (`self.DisableInput` (`GameplayStatics.GetPlayerController` 0)))

(event `Key|E`
  (params (Key :type "Key Structure"))
  (:`Pressed`
    (if (`self.colliding`)
      (bind (_direction _timer) (`Timeline|Timeline`)
        (:`Update`
          (`SceneComponent.K2_SetRelativeRotation` (`self.SceneCaptureComponent2D`) (`KismetMathLibrary.MakeRotator` 180.0 0.0 (* _timer 90.0)) false false)
          (`SceneComponent.K2_SetRelativeRotation` (`self.SM_Bld_Greenhouse_Door_01`) (`KismetMathLibrary.MakeRotator` 0.0 0.0 (* _timer -90.0)) false false)
          (if (not (`self.opened`))
            (`GameplayStatics.PlaySoundAtLocation` "/Game/creepy_opened_door.creepy_opened_door" (`SceneComponent.K2_GetComponentLocation` (`self.DefaultSceneRoot`)) (struct) 1.0 1.0 0.0 null null null null)
            (set `self.opened` true)))))))

(event `self.Box.OnComponentBeginOverlap`
  (params (OverlappedComponent :type "PrimitiveComponent Object Reference") (OtherActor :type "Actor Object Reference") (OtherComp :type "PrimitiveComponent Object Reference") (OtherBodyIndex :type Integer) (bFromSweep :type Boolean) (SweepResult :type "HitResult Structure (by ref)"))
  (cast `/Game/FirstPerson/Blueprints/BP_FirstPersonCharacter` OtherActor)
  (set `self.colliding` true))

(event `self.Box.OnComponentEndOverlap`
  (params (OverlappedComponent :type "PrimitiveComponent Object Reference") (OtherActor :type "Actor Object Reference") (OtherComp :type "PrimitiveComponent Object Reference") (OtherBodyIndex :type Integer))
  (cast `/Game/FirstPerson/Blueprints/BP_FirstPersonCharacter` OtherActor)
  (set `self.colliding` false))

(fn `UserConstructionScript`)