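; Entrance double-door actor that the player opens with E while inside its trigger box, with a creepy sound on first opening.
; Actor overlap toggles player input, while the box sets a Colliding flag only for BP_FirstPersonCharacter.
; The Door_anim timeline yaws the greenhouse door mesh and SceneCaptureComponent2D in opposite directions.
; The Opened flag limits the sound to one play, and no closing logic exists.
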(event `self.ReceiveBeginPlay`
  (set `self.opened` false)
  (set `self.colliding` false))

(event `self.ReceiveActorBeginOverlap`
  (params (OtherActor :type "Actor Object Reference"))
  (`self.EnableInput` (`GameplayStatics.GetPlayerController` 0)))

(event `self.ReceiveActorEndOverlap`
  (params (OtherActor :type "Actor Object Reference"))
  (`self.DisableInput` (`GameplayStatics.GetPlayerController` 0)))

(event `Key|E`
  (params (Key :type "Key Structure"))
  (:`Pressed`
    (if (`self.colliding`)
      (bind (_direction _timer) (`Timeline|door_anim`)
        (:`Update`
          (`SceneComponent.K2_SetRelativeRotation` (`self.SceneCaptureComponent2D`) (`KismetMathLibrary.MakeRotator` 0.0 0.0 (* _timer 87.0)) false false)
          (`SceneComponent.K2_SetRelativeRotation` (`self.SM_Bld_Greenhouse_Large_Door_02`) (`KismetMathLibrary.MakeRotator` 0.0 0.0 (* _timer -87.0)) false false)
          (if (not (`self.opened`))
            (`GameplayStatics.PlaySoundAtLocation` "/Game/creepy_opened_door.creepy_opened_door" (`SceneComponent.K2_GetComponentLocation` (`self.DefaultSceneRoot`)) (struct) 1.0 1.0 0.0 null null null null)
            (set `self.opened` true)))))))

(event `self.Box.OnComponentBeginOverlap`
  (params (OverlappedComponent :type "PrimitiveComponent Object Reference") (OtherActor :type "Actor Object Reference") (OtherComp :type "PrimitiveComponent Object Reference") (OtherBodyIndex :type Integer) (bFromSweep :type Boolean) (SweepResult :type "HitResult Structure (by ref)"))
  (cast `/Game/FirstPerson/Blueprints/BP_FirstPersonCharacter` OtherActor)
  (set `self.colliding` true))

(event `self.Box.OnComponentEndOverlap`
  (params (OverlappedComponent :type "PrimitiveComponent Object Reference") (OtherActor :type "Actor Object Reference") (OtherComp :type "PrimitiveComponent Object Reference") (OtherBodyIndex :type Integer))
  (cast `/Game/FirstPerson/Blueprints/BP_FirstPersonCharacter` OtherActor)
  (set `self.colliding` false))

(fn `UserConstructionScript`)